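; Quiz trigger actor that shows an AI-generated science multiple-choice question when the third-person character overlaps its sphere.
; Uses VaRest to POST to OpenRouter's DeepSeek model with a hardcoded API key and a JSON-only prompt.
; Decodes the nested reply into a quiz struct, setting the correct index from the loop index rather than answer_index.
; Passes the struct to WBP_Quiz and switches to UI-only input with the cursor shown.
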(event OnComponentBeginOverlap(Sphere1)
  (params (OverlappedComponent :type Primitive%20Component%20Object%20Reference) (OtherActor :type Actor%20Object%20Reference) (OtherComp :type Primitive%20Component%20Object%20Reference) (OtherBodyIndex :type Integer) (bFromSweep :type Boolean) (SweepResult :type Hit%20Result%20Structure%20%28by%20ref%29))
  (Utilities|Casting|CastToBP_ThirdPersonCharacter OtherActor)
  (CallFunction|GenerateQuizRequest))

(event Custom|GenerateQuiz_Request
  (bind _returnvalue (Class|VaRestSubsystem|ConstructVaRestRequestExt (|VaRestSubsystem) "POST" "json"))
  (Class|VaRestRequestJSON|SetURL _returnvalue "https://openrouter.ai/api/v1/chat/completions")
  (Class|VaRestRequestJSON|SetHeader _returnvalue "Authorization" "Bearer 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")
  (bind _returnvalue_2 (Class|VaRestSubsystem|ConstructVaRestJsonObject (|VaRestSubsystem)))
  (bind _output_get (Variables|Default|Setjson%20doc%20inner _returnvalue_2))
  (Class|VaRestJsonObject|SetStringField _output_get "model" "deepseek/deepseek-r1-0528:free")
  (Class|VaRestJsonObject|SetArrayField (Variables|Default|Getjson%20doc%20inner) "messages" (Utilities|Array|MakeArray (Class|VaRestSubsystem|ConstructJsonValueObject (|VaRestSubsystem) (|MakeJson "system" "You are a helpful assistant that answers strictly in JSON only. Never add any extra text, explanations, markdown, or code blocks. Respond with ONLY the requested JSON structure.")) (Class|VaRestSubsystem|ConstructJsonValueObject (|VaRestSubsystem) (|MakeJson "user" "Generate a multiple choice quiz question about science. 
 
Return ONLY a JSON object with this exact structure (no markdown, no extra text): 
{ 
\"question\": \"the question text here\", 
\"choices\": [\"choice A\", \"choice B\", \"choice C\", \"choice D\"], 
\"answer_index\": 0 
} 
 
The answer_index should be 0-3 indicating which choice is correct."))))
  (Class|VaRestRequestJSON|SetRequestObject _returnvalue (Variables|Default|Getjson%20doc%20inner))
  (Class|VaRestRequestJSON|ExecuteProcessRequest _returnvalue)
  (EventDispatchers|AssignOnRequestComplete _returnvalue (delegate Custom|OnRequestComplete_Event))
  (EventDispatchers|AssignOnRequestFail _returnvalue (delegate Custom|OnRequestFail_Event)))

(event Custom|OnRequestComplete_Event
  (params (Request :type Va%20Rest%20Request%20JSON%20Object%20Reference))
  (bind _returnvalue (Game|GetPlayerController 0))
  (bind _returnvalue_2 (Class|VaRestRequestJSON|GetResponseContentasString Request true))
  (bind _returnvalue_3 (Class|VaRestSubsystem|ConstructVaRestJsonObject (|VaRestSubsystem)))
  (Class|VaRestJsonObject|DecodeJson _returnvalue_3 _returnvalue_2 true)
  (bind _returnvalue_4 (Class|VaRestJsonValue|AsObject (Utilities|Array|Get(acopy) (Class|VaRestJsonObject|GetArrayField _returnvalue_3 "choices"))))
  (bind _returnvalue_5 (Class|VaRestSubsystem|ConstructVaRestJsonObject (|VaRestSubsystem)))
  (Class|VaRestJsonObject|DecodeJson _returnvalue_5 (Class|VaRestJsonObject|GetStringField (Class|VaRestJsonObject|GetObjectField _returnvalue_4 "message") "content") true)
  (Development|PrintString (Class|VaRestJsonObject|GetStringField _returnvalue_5 "question") true true "(R=0.000000,G=0.660000,B=1.000000,A=1.000000)" 1e+01)
  (for (_array_element _array_index) (Class|VaRestJsonObject|GetStringArrayField _returnvalue_5 "choices")
    (Development|PrintString _array_element true true "(R=0.000000,G=0.660000,B=1.000000,A=1.000000)" 1e+01)
    (Utilities|Struct|SetmembersinST_Quiz (Variables|Default|Getst_Quiz) (Class|VaRestJsonObject|GetStringField _returnvalue_5 "question") (Class|VaRestJsonObject|GetStringArrayField _returnvalue_5 "choices") _array_index))
  (bind _returnvalue_6 (UserInterface|CreateWidget "/Game/Quiz/WBP_Quiz.WBP_Quiz_C" 0 (Variables|Default|Getst_Quiz)))
  (bind _output_get (Variables|Default|SetQuizWidgetRef _returnvalue_6))
  (UserInterface|Viewport|AddtoViewport _returnvalue_6 0)
  (Variables|/Script/Engine.PlayerController|SetbShowMouseCursor _returnvalue true)
  (Input|SetInputModeUIOnly _returnvalue _output_get "DoNotLock" false))

(event Custom|OnRequestFail_Event
  (params (Request :type Va%20Rest%20Request%20JSON%20Object%20Reference))
  (Utilities|FlowControl|DoOnce false
    (:Completed
      (bind _returnvalue (Class|VaRestRequestJSON|GetResponseContentasString Request true))
      (Development|PrintString _returnvalue true true "(R=0.000000,G=0.660000,B=1.000000,A=1.000000)" 1e+01))))

(event Collision|EventActorBeginOverlap
  (params (OtherActor :type Actor%20Object%20Reference)))

(event EventTick
  (params (DeltaSeconds :type Float%20%28single-precision%29)))

(fn ConstructionScript)